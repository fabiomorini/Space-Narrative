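; BP_Alien is an enemy AI character that wanders at random and chases the first-person player on sight.
; A self-calling patrol event waits a random delay, then moves to a random reachable navmesh point while the player is unseen.
; PawnSensing sightings raise walk speed and start an AI move toward the player.
; A retriggerable delay, refreshed by each sighting, clears the seen flag after TimeToLoseTrack and resumes patrol.
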(event `self.ReceiveBeginPlay`
  (`self.PatrolRandom`))

(event `PatrolRandom`
  (set `CharacterMovementComponent.MaxWalkSpeed` 300.0 (`self.CharacterMovement`))
  (`KismetSystemLibrary.Delay` (`KismetMathLibrary.RandomFloatInRange` 6.0 12.0))
  (if (not (`self.CanSeePlayer?`))
    (`|AIMoveTo` self (`NavigationSystemV1.K2_GetRandomReachablePointInRadius` (`self.K2_GetActorLocation`) 30000.0 null null) null
      (:`then`
        _)
      (:`OnSuccess`
        _)
      (:`OnFail`
        _))
    (`self.PatrolRandom`)))

(event `self.PawnSensing.OnSeePawn`
  (params (Pawn :type "Pawn Object Reference"))
  (bind _asbp_first_person_character (cast `/Game/FirstPerson/Blueprints/BP_FirstPersonCharacter` Pawn))
  (`|ExecutionSequence`
    (:`then_0`
      (set `self.CanSeePlayer?` true)
      (set `CharacterMovementComponent.MaxWalkSpeed` 450.0 (`self.CharacterMovement`))
      (`|AIMoveTo` self (0.0 0.0 0.0) _asbp_first_person_character))
    (:`then_1`
      (`KismetSystemLibrary.RetriggerableDelay` (`self.TimeToLoseTrack`))
      (set `self.CanSeePlayer?` false)
      (`self.PatrolRandom`))))

(event `self.PawnSensing.OnHearNoise`
  (params (Instigator :type "Pawn Object Reference") (Location :type "Vector Structure (by ref)") (Volume :type "Float (single-precision)")))

(fn `UserConstructionScript`)
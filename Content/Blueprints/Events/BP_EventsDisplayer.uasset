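; BP_EventsDisplayer is a Blueprint that shows event tasks on an in-world control panel screen.
; Its CreateTask and DeleteTask events fetch the user widget from the Screen component and cast it to WBP_ControlPanel.
; Each event then forwards the task to the panel's WBPTaskList to add or remove it, doing nothing if the cast fails.
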(event `CreateTask`
  (params (TaskToCreate :type "/Game/Blueprints/E_RandomEvents Enum" :default "NewEnumerator0"))
  (bind _aswbp_control_panel (cast `/Game/Blueprints/WBP_ControlPanel` (`WidgetComponent.GetUserWidgetObject` (`self.Screen`))))
  (`/Game/Blueprints/WBP_TaskList.CreateTask` (`/Game/Blueprints/WBP_ControlPanel.WBP_TaskList` _aswbp_control_panel) TaskToCreate))

(event `DeleteTask`
  (params (TaskToDelete :type "/Game/Blueprints/E_RandomEvents Enum" :default "NewEnumerator0"))
  (bind _aswbp_control_panel (cast `/Game/Blueprints/WBP_ControlPanel` (`WidgetComponent.GetUserWidgetObject` (`self.Screen`))))
  (`/Game/Blueprints/WBP_TaskList.DeleteTask` (`/Game/Blueprints/WBP_ControlPanel.WBP_TaskList` _aswbp_control_panel) TaskToDelete))

(fn `UserConstructionScript`)
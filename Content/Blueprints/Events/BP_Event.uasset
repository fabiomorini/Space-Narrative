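; Interactable task actor that, once activated, shows a custom-depth outline and starts a fail timer.
; Inside its box, the player holds Interact through a repair timer, with a progress widget, sound and locked movement.
; Co-op tasks also activate a linked partner and complete when Tick finds both held within a short window.
; Completion or failure updates GameMode tallies (half per co-op task) and clears the active event.
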(event `self.ReceiveBeginPlay`
  ;[1 1 1] Outline Color
  (`PrimitiveComponent.SetCustomDepthStencilValue` (`self.StaticMesh`) (`BlueprintMapLibrary.Map_Find` (`self.OutlineColorMap`) (`self.OutlineColor`))))

(event `TaskFailed`
  ;[1 1 1] TASK FAILED
  (if (not (`self.Completed`))
    (bind _asbp_first_person_game_mode (cast `/Game/FirstPerson/Blueprints/BP_FirstPersonGameMode` (`GameplayStatics.GetGameMode`)))
    (if (`self.IsCoopTask`)
      (set `/Game/FirstPerson/Blueprints/BP_FirstPersonGameMode.TasksFailed` (+ (`/Game/FirstPerson/Blueprints/BP_FirstPersonGameMode.TasksFailed` _asbp_first_person_game_mode) 0.5) _asbp_first_person_game_mode)
      (else
        (set `/Game/FirstPerson/Blueprints/BP_FirstPersonGameMode.TasksFailed` (+ (`/Game/FirstPerson/Blueprints/BP_FirstPersonGameMode.TasksFailed` _asbp_first_person_game_mode) 1.0) _asbp_first_person_game_mode)))
    (bind _activeevents (`/Game/FirstPerson/Blueprints/BP_FirstPersonGameMode.ActiveEvents` _asbp_first_person_game_mode))
    (`KismetArrayLibrary.Array_Remove` _activeevents (`KismetArrayLibrary.Array_Find` _activeevents (`self.Event`)))
    (bind _asbp_first_person_game_mode_2 (cast `/Game/FirstPerson/Blueprints/BP_FirstPersonGameMode` (`GameplayStatics.GetGameMode`)))
    (`/Game/FirstPerson/Blueprints/BP_FirstPersonGameMode.CompleteTask` _asbp_first_person_game_mode_2 (`self.Event`))
    (set `self.Activated` false)
    (`PrimitiveComponent.SetRenderCustomDepth` (`self.StaticMesh`) false)
    (`/Game/FirstPerson/Blueprints/BP_FirstPersonGameMode.EndGame` _asbp_first_person_game_mode_2)))

(event `TaskCompleted`
  ;[1 1 1] TASK COMPLETED
  (`/Engine/EditorBlueprintResources/StandardMacros.DoOnce` false :!label _label
    (:`Completed`
      (`PrimitiveComponent.SetRenderCustomDepth` (`self.StaticMesh`) false)
      (`KismetSystemLibrary.PrintString` "TASK COMPLETED" true true (struct :`R` 0.004252 :`G` 1.0 :`A` 1.0) 40.0)
      (set `self.Completed` true)
      (bind _asbp_first_person_game_mode (cast `/Game/FirstPerson/Blueprints/BP_FirstPersonGameMode` (`GameplayStatics.GetGameMode`)))
      (if (`self.IsCoopTask`)
        (set `/Game/FirstPerson/Blueprints/BP_FirstPersonGameMode.TasksEnded` (+ (`/Game/FirstPerson/Blueprints/BP_FirstPersonGameMode.TasksEnded` _asbp_first_person_game_mode) 0.5) _asbp_first_person_game_mode)
        (else
          (set `/Game/FirstPerson/Blueprints/BP_FirstPersonGameMode.TasksEnded` (+ (`/Game/FirstPerson/Blueprints/BP_FirstPersonGameMode.TasksEnded` _asbp_first_person_game_mode) 1.0) _asbp_first_person_game_mode)))
      (bind _activeevents (`/Game/FirstPerson/Blueprints/BP_FirstPersonGameMode.ActiveEvents` _asbp_first_person_game_mode))
      (`KismetArrayLibrary.Array_Remove` _activeevents (`KismetArrayLibrary.Array_Find` _activeevents (`self.Event`)))
      (bind _asbp_first_person_game_mode_2 (cast `/Game/FirstPerson/Blueprints/BP_FirstPersonGameMode` (`GameplayStatics.GetGameMode`)))
      (`/Game/FirstPerson/Blueprints/BP_FirstPersonGameMode.CompleteTask` _asbp_first_person_game_mode_2 (`self.Event`))
      (set `self.Activated` false)
      (`ActorComponent.Activate` (`Character.CharacterMovement` (`self.Player`)) false)
      (bind _repairsound (`self.RepairSound`)
        (:`then`
          (`AudioComponent.Stop` _repairsound)
          (`/Game/FirstPerson/Blueprints/BP_FirstPersonGameMode.EndGame` _asbp_first_person_game_mode_2))
        (:`else`)))))

(event `ResetInteract`
  ;[1 1 1] TASK COMPLETED
  (goto _label :!via `Reset`))

(event `/Game/Blueprints/BPI_Interact.ActivateEvent`
  (params (Event :type "/Game/Blueprints/E_RandomEvents Enum" :default "NewEnumerator0"))
  ;[1 1 1] CREATE TASK
  (bind _output_get (set `self.ActiveEvent` Event))
  (if (`|EnumEquality` _output_get (`self.Event`))
    (bind _returnvalue (`KismetSystemLibrary.K2_SetTimerDelegate` (`|CreateDelegate` :!event `TaskFailed`) (`self.TimeToFailTask`)))
    (`self.ResetInteract`)
    (`PrimitiveComponent.SetRenderCustomDepth` (`self.StaticMesh`) true)
    (set `self.Activated` true)
    (set `self.Completed` false)
    (set `self.CoopCheck` false)
    (if (`self.IsCoopTask`)
      (bind _taskcoop (`self.TaskCoop`)
        (:`then`
          (if (not (`/Game/Blueprints/Events/BP_Event.Activated` _taskcoop))
            (`/Game/Blueprints/BPI_Interact.ActivateEvent` _taskcoop (`self.Event`))))
        (:`else`)))))

(event `StopTimer`
  ;[1 1 1] CREATE TASK
  (`KismetSystemLibrary.K2_PauseTimerHandle` (stale `RepairTimer` _returnvalue) :!label _label_2))

(event `EndGame`
  ;[1 1 1] CREATE TASK
  (`KismetSystemLibrary.K2_ClearAndInvalidateTimerHandle` (stale `/Game/Blueprints/BPI_Interact.ActivateEvent` _returnvalue))
  (goto _label_2))

(event `self.Box.OnComponentBeginOverlap`
  (params (OverlappedComponent :type "PrimitiveComponent Object Reference") (OtherActor :type "Actor Object Reference") (OtherComp :type "PrimitiveComponent Object Reference") (OtherBodyIndex :type Integer) (bFromSweep :type Boolean) (SweepResult :type "HitResult Structure (by ref)"))
  ;[1 1 1] INTERACT WITH TASK
  (bind _asbp_first_person_character (cast `/Game/FirstPerson/Blueprints/BP_FirstPersonCharacter` OtherActor))
  (set `self.Player` _asbp_first_person_character)
  (if (`self.Activated`)
    (set `self.IsHeld?` false)
    (`self.EnableInput` (`GameplayStatics.GetPlayerController` 0))
    (`self.ResetInteract`)
    (bind _returnvalue (`|CreateWidget` "/Game/Blueprints/Events/WBP_Repair.WBP_Repair_C"))
    (bind _output_get (set `self.RepairWidgetRef` _returnvalue))
    (`UserWidget.AddToViewport` _output_get 0)
    (goto _label_3 :!via `Open`)))

(event `InputAction|Interact`
  (params (Key :type "Key Structure"))
  (bind _charactermovement (`Character.CharacterMovement` (`self.Player`)))
  ;[1 1 1] INTERACT WITH TASK
  (:`Pressed`
    (`ActorComponent.Deactivate` _charactermovement)
    (set `self.IsHeld?` true)
    (`KismetSystemLibrary.K2_PauseTimerHandle` (stale `RepairTimer` _returnvalue))
    (`/Engine/EditorBlueprintResources/StandardMacros.Gate` true :!label _label_3
      (:`Exit`
        (`|ExecutionSequence`
          (:`then_0`
            (`KismetSystemLibrary.RetriggerableDelay` (`self.MaxHoldTime`))
            (if (`self.IsHeld?`)
              (`Widget.RemoveFromParent` (`self.RepairWidgetRef`))
              (if (not (`self.IsCoopTask`))
                (`self.TaskCompleted`)
                (else
                  (set `self.CoopCheck` true)
                  (`KismetSystemLibrary.RetriggerableDelay` (`self.TimeInBetweenCoopTasks`))
                  (set `self.CoopCheck` false)))))
          (:`then_1`
            (`self.RepairTimer`)
            (`self.UpdateTimer`))
          (:`then_2`
            (bind _returnvalue (`GameplayStatics.CreateSound2D` "/Game/Blueprints/Events/RepairSound.RepairSound" 1.0 1.0 0.0 null))
            (bind _output_get (set `self.RepairSound` _returnvalue))
            (`AudioComponent.Play` _output_get 0.0))))))
  (:`Released`
    (`ActorComponent.Activate` _charactermovement false)
    (set `self.IsHeld?` false)
    (`KismetSystemLibrary.K2_UnPauseTimerHandle` (stale `RepairTimer` _returnvalue))
    (bind _repairsound (`self.RepairSound`)
      (:`then`
        (`AudioComponent.Stop` _repairsound))
      (:`else`))))

(event `self.Box.OnComponentEndOverlap`
  (params (OverlappedComponent :type "PrimitiveComponent Object Reference") (OtherActor :type "Actor Object Reference") (OtherComp :type "PrimitiveComponent Object Reference") (OtherBodyIndex :type Integer))
  ;[1 1 1] INTERACT WITH TASK
  (cast `/Game/FirstPerson/Blueprints/BP_FirstPersonCharacter` OtherActor)
  (if (`self.Activated`)
    (`self.DisableInput` (`GameplayStatics.GetPlayerController` 0))
    (bind _repairwidgetref (`self.RepairWidgetRef`)
      (:`then`
        (`Widget.RemoveFromParent` _repairwidgetref)
        (set `/Game/Blueprints/Events/WBP_Repair.TimeHeld` 0.0 _repairwidgetref))
      (:`else`
        _))
    (set `self.IsHeld?` false)
    (`self.StopTimer`)
    (goto _label_3 :!via `Close`)))

(event `self.ReceiveTick`
  (params (DeltaSeconds :type "Float (single-precision)"))
  ;[1 1 1] CheckTaskCoop
  (if (`self.IsCoopTask`)
    (if (`self.CoopCheck`)
      (bind _taskcoop (`self.TaskCoop`)
        (:`then`
          (if (`/Game/Blueprints/Events/BP_Event.CoopCheck` _taskcoop)
            (`self.TaskCompleted`)))
        (:`else`)))))

(event `RepairTimer`
  ;[1 1 1] REPAIR TIMER
  (bind _returnvalue (`KismetSystemLibrary.K2_SetTimerDelegate` (delegate `RepairTimer`) (`self.MaxHoldTime`))))

(event `UpdateTimer`
  (bind _repairwidgetref (`self.RepairWidgetRef`))
  ;[1 1 1] REPAIR TIMER
  (if (`self.IsHeld?`)
    (set `/Game/Blueprints/Events/WBP_Repair.TimeHeld` (`KismetSystemLibrary.K2_GetTimerElapsedTimeHandle` (stale `RepairTimer` _returnvalue)) _repairwidgetref)
    (`KismetSystemLibrary.Delay` 0.01)
    (`self.UpdateTimer`)
    (else
      (`self.StopTimer`)
      (set `/Game/Blueprints/Events/WBP_Repair.TimeHeld` 0.0 _repairwidgetref))))

(fn `UserConstructionScript`
  (bind _staticmesh (`self.StaticMesh`))
  (switch `/Game/Blueprints/E_RandomEvents` (`self.Event`)
    (:`NewEnumerator0`
      _)
    (:`NewEnumerator1`
      _)
    (:`NewEnumerator2`
      _)
    (:`NewEnumerator3`
      _)
    (:`NewEnumerator4`
      _)
    (:`NewEnumerator5`
      _)
    (:`NewEnumerator6`
      (`StaticMeshComponent.SetStaticMesh` _staticmesh "/Engine/BasicShapes/Cube.Cube")
      (`PrimitiveComponent.SetMaterial` _staticmesh 0 "/Engine/EngineMeshes/BackgroundMaterial.BackgroundMaterial")))
  (`PrimitiveComponent.SetRenderCustomDepth` (`self.StaticMesh`) false))
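; Motor event actor, a child of an event Blueprint, that spins four rotators and shows a beam while working, which it does from BeginPlay.
; Tick watches event state: Activated stops the motor, while Completed without Activated restarts it.
; The Rotators timeline eases spin up or down around three-second delays.
; Paired DoOnce gates re-arm each other so each transition fires once.
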(event `self.ReceiveBeginPlay`
  (set `self.Working` true)
  (`SceneComponent.SetVisibility` (`self.P_beam`) false false))

(event `ResetStopMotor`
  (goto _label :!via `Reset`))

(event `self.ReceiveTick`
  (params (DeltaSeconds :type "Float (single-precision)"))
  (`parent.ReceiveTick` DeltaSeconds)
  (`|ExecutionSequence`
    (:`then_0`
      (if (`self.Activated`)
        (`/Engine/EditorBlueprintResources/StandardMacros.DoOnce` false :!label _label
          (:`Completed`
            (set `self.Working` false)
            (`self.StopRotators`)
            (`KismetSystemLibrary.Delay` 3.0)
            (`self.ResetMoveMotor`)
            (`SceneComponent.SetVisibility` (`self.P_beam`) false false)))
        (elif (`self.Completed`)
          (`/Engine/EditorBlueprintResources/StandardMacros.DoOnce` false :!label _label_2
            (:`Completed`
              (`self.ActivateRotators`)
              (`KismetSystemLibrary.Delay` 3.0)
              (set `self.Working` true)
              (`self.ResetStopMotor`))))))
    (:`then_1`
      (if (`self.Working`)
        (`SceneComponent.K2_AddLocalRotation` (`self.Rotator1`) (`KismetMathLibrary.MakeRotator` 10.0) false false)
        (`SceneComponent.K2_AddLocalRotation` (`self.Rotator3`) (`KismetMathLibrary.MakeRotator` 10.0) false false)
        (`SceneComponent.K2_AddLocalRotation` (`self.Rotator4`) (`KismetMathLibrary.MakeRotator` 10.0) false false)
        (`SceneComponent.K2_AddLocalRotation` (`self.Rotator2`) (`KismetMathLibrary.MakeRotator` 10.0) false false)
        (`SceneComponent.SetVisibility` (`self.P_beam`) true false)))))

(event `ResetMoveMotor`
  (goto _label_2 :!via `Reset`))

(event `ActivateRotators`
  (bind (_direction _alpha) (`Timeline|Rotators` :!via `PlayFromStart` :!label _label_3)
    (:`Update`
      (`SceneComponent.K2_AddLocalRotation` (`self.Rotator1`) (`KismetMathLibrary.MakeRotator` _alpha) false false)
      (`SceneComponent.K2_AddLocalRotation` (`self.Rotator3`) (`KismetMathLibrary.MakeRotator` _alpha) false false)
      (`SceneComponent.K2_AddLocalRotation` (`self.Rotator4`) (`KismetMathLibrary.MakeRotator` _alpha) false false)
      (`SceneComponent.K2_AddLocalRotation` (`self.Rotator2`) (`KismetMathLibrary.MakeRotator` _alpha) false false))))

(event `StopRotators`
  (goto _label_3 :!via `ReverseFromEnd`))

(fn `UserConstructionScript`
  (`parent.UserConstructionScript`)
  (`StaticMeshComponent.SetStaticMesh` (`self.StaticMesh`) "/Game/ScienceLab/Meshes/ScientificDevice/GasDynamicTrap/SM_GasDynamicTrap1.SM_GasDynamicTrap1"))
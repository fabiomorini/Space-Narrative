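; Child event Blueprint for a water tank prop that drains and refills by moving its water mesh vertically.
; While Activated, Tick starts the drain through a DoOnce gate, and also the fill through a second gate if IsHeld.
; Each timeline adds lerped relative Z offsets per update, and on finishing resets the opposite action's gate.
; The construction script sets the scientific device mesh.
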(event `self.ReceiveBeginPlay`
  (set `self.WaterPosition` 2.5))

(event `RestartWaterEmpty`
  (goto _label :!via `Reset`))

(event `self.ReceiveTick`
  (params (DeltaSeconds :type "Float (single-precision)"))
  (`parent.ReceiveTick` DeltaSeconds)
  (if (`self.Activated`)
    (`|ExecutionSequence`
      (:`then_0`
        (`/Engine/EditorBlueprintResources/StandardMacros.DoOnce` false :!label _label
          (:`Completed`
            (`self.EmptyWaterTank`))))
      (:`then_1`
        (if (`self.IsHeld?`)
          (`/Engine/EditorBlueprintResources/StandardMacros.DoOnce` false :!label _label_2
            (:`Completed`
              (`self.FillWaterTank`))))))))

(event `RestartWaterFill`
  (goto _label_2 :!via `Reset`))

(event `EmptyWaterTank`
  (bind (_direction _alpha) (`Timeline|WaterMove` :!via `PlayFromStart`)
    (:`Update`
      (`SceneComponent.K2_AddRelativeLocation` (`self.StaticMeshWater`) (`KismetMathLibrary.VLerp` (0.0 0.0 0.0) (`KismetMathLibrary.MakeVector` 0.0 0.0 (* (`self.WaterPosition`) -1.0)) _alpha) false false))
    (:`Finished`
      (`self.RestartWaterFill`))))

(event `FillWaterTank`
  (bind (_direction _alpha) (`Timeline|Timeline_0` :!via `PlayFromStart`)
    (:`Update`
      (if (`self.IsHeld?`)
        _
        (else
          _))
      (`SceneComponent.K2_AddRelativeLocation` (`self.StaticMeshWater`) (`KismetMathLibrary.VLerp` (`KismetMathLibrary.MakeVector` 0.0 0.0 (`self.WaterPosition`)) (0.0 0.0 0.0) _alpha) false false))
    (:`Finished`
      (`self.RestartWaterEmpty`))))

(fn `UserConstructionScript`
  (`parent.UserConstructionScript`)
  (`StaticMeshComponent.SetStaticMesh` (`self.StaticMesh`) "/Game/ScienceLab/Meshes/ScientificDevice/SM_ScientificDevice03.SM_ScientificDevice03"))
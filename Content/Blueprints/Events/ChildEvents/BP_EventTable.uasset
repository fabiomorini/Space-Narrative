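; BP_EventTable is a child event actor for a table whose two doors swing when the event is activated and held.
; Tick checks the Activated and IsHeld flags, then fires MoveDoors through a DoOnce.
; Two timelines yaw Door1 and Door2 in relative space, with the second alpha negated.
; When they finish, a shared one-second delay resets the DoOnce, so the motion can repeat.
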(event `self.ReceiveTick`
  (params (DeltaSeconds :type "Float (single-precision)"))
  (`parent.ReceiveTick` DeltaSeconds)
  (if (`self.Activated`)
    (if (`self.IsHeld?`)
      (`/Engine/EditorBlueprintResources/StandardMacros.DoOnce` false :!label _label
        (:`Completed`
          (`self.MoveDoors`))))))

(event `ResetMovement`
  (goto _label :!via `Reset`))

(event `MoveDoors`
  (`|ExecutionSequence`
    (:`then_0`
      (bind (_direction _alpha) (`Timeline|MoveDoor1` :!via `PlayFromStart`)
        (:`Update`
          (`SceneComponent.K2_SetRelativeRotation` (`self.Door1`) (`KismetMathLibrary.MakeRotator` 0.0 0.0 _alpha) false false))
        (:`Finished`
          (`KismetSystemLibrary.Delay` 1.0 :!label _label_2)
          (`self.ResetMovement`))))
    (:`then_1`
      (bind (_direction_2 _alpha_2) (`Timeline|MoveDoor2` :!via `PlayFromStart`)
        (:`Update`
          (`SceneComponent.K2_SetRelativeRotation` (`self.Door2`) (`KismetMathLibrary.MakeRotator` 0.0 0.0 (* _alpha_2 -1.0)) false false))
        (:`Finished`
          (goto _label_2))))))

(fn `UserConstructionScript`
  (`parent.UserConstructionScript`)
  (`StaticMeshComponent.SetStaticMesh` (`self.StaticMesh`) "/Game/ScienceLab/Meshes/Furniture/SM_Table03.SM_Table03"))
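; Child event Blueprint for a filing cabinet prop that slides its three boxes along local Y while it is activated and held.
; Tick checks both flags and passes through a DoOnce into MoveCabinets, which starts three timelines together, one per box.
; Timeline completion leads to a one-second delay that resets the DoOnce, so the motion repeats while the conditions hold.
; The construction script assigns the filing cabinet mesh.
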(event `self.ReceiveTick`
  (params (DeltaSeconds :type "Float (single-precision)"))
  (`parent.ReceiveTick` DeltaSeconds)
  (if (`self.Activated`)
    (if (`self.IsHeld?`)
      (`/Engine/EditorBlueprintResources/StandardMacros.DoOnce` false :!label _label
        (:`Completed`
          (`self.MoveCabinets`))))))

(event `ResetMovement`
  (goto _label :!via `Reset`))

(event `MoveCabinets`
  (`|ExecutionSequence`
    (:`then_0`
      (bind (_direction _alpha) (`Timeline|MoveTimeline1` :!via `PlayFromStart`)
        (:`Update`
          (`SceneComponent.K2_SetRelativeLocation` (`self.Box1`) (`KismetMathLibrary.MakeVector` 0.0 _alpha 70.161964) false false))
        (:`Finished`
          (`KismetSystemLibrary.Delay` 1.0 :!label _label_2)
          (`self.ResetMovement`))))
    (:`then_1`
      (bind (_direction_2 _alpha_2) (`Timeline|MoveTimeline2` :!via `PlayFromStart`)
        (:`Update`
          (`SceneComponent.K2_SetRelativeLocation` (`self.Box2`) (`KismetMathLibrary.MakeVector` 0.0 _alpha_2 40.122208) false false))
        (:`Finished`
          (goto _label_2))))
    (:`then_2`
      (bind (_direction_3 _alpha_3) (`Timeline|MoveTimeline3` :!via `PlayFromStart`)
        (:`Update`
          (`SceneComponent.K2_SetRelativeLocation` (`self.Box3`) (`KismetMathLibrary.MakeVector` 0.0 _alpha_3 10.082724) false false))
        (:`Finished`
          (goto _label_2))))))

(fn `UserConstructionScript`
  (`parent.UserConstructionScript`)
  (`StaticMeshComponent.SetStaticMesh` (`self.StaticMesh`) "/Game/ScienceLab/Meshes/OfficeProps/SM_FilingCabinets1.SM_FilingCabinets1"))
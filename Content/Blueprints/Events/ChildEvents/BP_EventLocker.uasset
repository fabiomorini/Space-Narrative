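; Locker event actor, a child event Blueprint that animates two doors and a drawer while activated and held.
; Tick passes through a DoOnce to MoveParts, which starts three timelines together to yaw the doors with opposite signs and slide the drawer along Y.
; Timeline completions share a one-second Delay that resets the DoOnce, so the motion replays from the start while both conditions hold.
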(event `self.ReceiveTick`
  (params (DeltaSeconds :type "Float (single-precision)"))
  (`parent.ReceiveTick` DeltaSeconds)
  (if (`self.Activated`)
    (if (`self.IsHeld?`)
      (`/Engine/EditorBlueprintResources/StandardMacros.DoOnce` false :!label _label
        (:`Completed`
          (`self.MoveParts`))))))

(event `ResetMovement`
  (goto _label :!via `Reset`))

(event `MoveParts`
  (`|ExecutionSequence`
    (:`then_0`
      (bind (_direction _alpha) (`Timeline|MovePart1` :!via `PlayFromStart`)
        (:`Update`
          (`SceneComponent.K2_SetRelativeRotation` (`self.Door1`) (`KismetMathLibrary.MakeRotator` 0.0 0.0 _alpha) false false))
        (:`Finished`
          (`KismetSystemLibrary.Delay` 1.0 :!label _label_2)
          (`self.ResetMovement`))))
    (:`then_1`
      (bind (_direction_2 _alpha_2) (`Timeline|MovePart2` :!via `PlayFromStart`)
        (:`Update`
          (`SceneComponent.K2_SetRelativeRotation` (`self.Door2`) (`KismetMathLibrary.MakeRotator` 0.0 0.0 (* _alpha_2 -1.0)) false false))
        (:`Finished`
          (goto _label_2))))
    (:`then_2`
      (bind (_direction_3 _alpha_3) (`Timeline|MovePart3` :!via `PlayFromStart`)
        (:`Update`
          (`SceneComponent.K2_SetRelativeLocation` (`self.Drawer`) (`KismetMathLibrary.MakeVector` 0.0 (+ (* _alpha_3 -1.0) -50.0) 79.608948) false false))
        (:`Finished`
          (goto _label_2))))))

(fn `UserConstructionScript`
  (`parent.UserConstructionScript`)
  (`StaticMeshComponent.SetStaticMesh` (`self.StaticMesh`) "/Game/ScienceLab/Meshes/Furniture/SM_Locker05.SM_Locker05"))
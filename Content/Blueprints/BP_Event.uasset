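; BP_Event is an interactable task object whose Event type picks its mesh and material in the Construction Script.
; ActivateEvent arms a matching task with a custom-depth highlight, and the Box overlap then enables player input and resets the DoOnce.
; Interact clears the highlight and text, updates TasksEnded and ActiveEvents on BP_FirstPersonGameMode, and swaps broken tanks to intact ones.
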(event `InputAction|Interact`
  (params (Key :type "Key Structure"))
  (:`Pressed`
    (`/Engine/EditorBlueprintResources/StandardMacros.DoOnce` false :!label _label
      (:`Completed`
        (`PrimitiveComponent.SetRenderCustomDepth` (`self.StaticMesh`) false)
        (`KismetSystemLibrary.PrintString` "TASK COMPLETED" true true (struct :`R` 0.004252 :`G` 1.0 :`A` 1.0) 40.0)
        (`SceneComponent.SetVisibility` (`self.TextRender`) false false)
        (bind _asbp_first_person_game_mode (cast `/Game/FirstPerson/Blueprints/BP_FirstPersonGameMode` (`GameplayStatics.GetGameMode`)))
        (`/Engine/EditorBlueprintResources/StandardMacros.IncrementInt` (`/Game/FirstPerson/Blueprints/BP_FirstPersonGameMode.TasksEnded` _asbp_first_person_game_mode)
          (:`  `
            (bind _activeevents (`/Game/FirstPerson/Blueprints/BP_FirstPersonGameMode.ActiveEvents` _asbp_first_person_game_mode))
            (`KismetArrayLibrary.Array_Remove` _activeevents (`KismetArrayLibrary.Array_Find` _activeevents (`self.Event`)))
            (if (or (`|EnumEquality` (`self.Event`) "NewEnumerator0") (`|EnumEquality` (`self.Event`) "NewEnumerator1"))
              (`StaticMeshComponent.SetStaticMesh` (`self.StaticMesh`) "/Game/Polar/Meshes/Props/SM_Tank.SM_Tank"))))))))

(event `ResetInteract`
  (goto _label :!via `Reset`))

(event `/Game/Blueprints/BPI_Interact.ActivateEvent`
  (params (Event :type "/Game/Blueprints/E_RandomEvents Enum" :default "NewEnumerator0"))
  (set `self.ActiveEvent` Event)
  (if (`|EnumEquality` Event (`self.Event`))
    (`PrimitiveComponent.SetRenderCustomDepth` (`self.StaticMesh`) true)
    (set `self.Activated` true)))

(event `self.Box.OnComponentBeginOverlap`
  (params (OverlappedComponent :type "PrimitiveComponent Object Reference") (OtherActor :type "Actor Object Reference") (OtherComp :type "PrimitiveComponent Object Reference") (OtherBodyIndex :type Integer) (bFromSweep :type Boolean) (SweepResult :type "HitResult Structure (by ref)"))
  (bind _asbp_first_person_character (cast `/Game/FirstPerson/Blueprints/BP_FirstPersonCharacter` OtherActor))
  (set `self.Player` _asbp_first_person_character)
  (if (`self.Activated`)
    (`self.EnableInput` (`GameplayStatics.GetPlayerController` 0))
    (`self.ResetInteract`)))

(event `self.Box.OnComponentEndOverlap`
  (params (OverlappedComponent :type "PrimitiveComponent Object Reference") (OtherActor :type "Actor Object Reference") (OtherComp :type "PrimitiveComponent Object Reference") (OtherBodyIndex :type Integer))
  (cast `/Game/FirstPerson/Blueprints/BP_FirstPersonCharacter` OtherActor)
  (`self.DisableInput` (`GameplayStatics.GetPlayerController` 0)))

(fn `UserConstructionScript`
  (bind _staticmesh (`self.StaticMesh`))
  (bind _staticmesh_2 (`self.StaticMesh`))
  (bind _staticmesh_3 (`self.StaticMesh`))
  (bind _staticmesh_4 (`self.StaticMesh`))
  (bind _staticmesh_5 (`self.StaticMesh`))
  (switch `/Game/Blueprints/E_RandomEvents` (`self.Event`)
    (:`NewEnumerator0`
      (`StaticMeshComponent.SetStaticMesh` (`self.StaticMesh`) "/Game/Polar/Meshes/Props/SM_Tank_Broken.SM_Tank_Broken" :!label _label))
    (:`NewEnumerator1`
      (goto _label))
    (:`NewEnumerator2`
      (`StaticMeshComponent.SetStaticMesh` _staticmesh_3 "/Game/Polar/Meshes/Architecture/SM_Pillar.SM_Pillar")
      (`PrimitiveComponent.SetMaterial` _staticmesh_3 0 "/Game/Polar/Materials/Architectural/M_Wall_Chrome_Inst.M_Wall_Chrome_Inst"))
    (:`NewEnumerator3`
      (`StaticMeshComponent.SetStaticMesh` _staticmesh_4 "/Engine/BasicShapes/Cube.Cube")
      (`PrimitiveComponent.SetMaterial` _staticmesh_4 0 "/AnimationSharing/AnimSharingGreen.AnimSharingGreen"))
    (:`NewEnumerator4`
      (`StaticMeshComponent.SetStaticMesh` _staticmesh_5 "/Engine/BasicShapes/Cube.Cube")
      (`PrimitiveComponent.SetMaterial` _staticmesh_5 0 "/Engine/MapTemplates/Materials/BasicAsset01.BasicAsset01"))
    (:`NewEnumerator5`
      (`StaticMeshComponent.SetStaticMesh` _staticmesh_2 "/Engine/BasicShapes/Cube.Cube")
      (`PrimitiveComponent.SetMaterial` _staticmesh_2 0 "/AnimationSharing/AnimSharingRed.AnimSharingRed"))
    (:`NewEnumerator6`
      (`StaticMeshComponent.SetStaticMesh` _staticmesh "/Engine/BasicShapes/Cube.Cube")
      (`PrimitiveComponent.SetMaterial` _staticmesh 0 "/Engine/EngineMeshes/BackgroundMaterial.BackgroundMaterial")))
  (`PrimitiveComponent.SetRenderCustomDepth` (`self.StaticMesh`) false))